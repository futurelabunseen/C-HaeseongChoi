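; BP_MonsterSpawner is an actor that periodically spawns random monsters at its own location.
; The construction script fills the class array with four monster types: Scorobey, Creepster, LandBug and Kraken.
; Tick accumulates delta time and, once it exceeds SpawnInterval, resets it and spawns a randomly picked class from that array.
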(event `self.ReceiveTick`
  (params (DeltaSeconds :type "Float (single-precision)"))
  (bind _output_get (set `self.DeltaSeconds` (+ DeltaSeconds (`self.DeltaSeconds`))))
  (if (> _output_get (`self.SpawnInterval`))
    (set `self.DeltaSeconds` 0.0)
    (`|SpawnActorFromClass` (`KismetArrayLibrary.Array_Random` (`self.MonsterClassArray`)) (`KismetMathLibrary.MakeTransform` (`self.K2_GetActorLocation`)) "Undefined" "MultiplyWithRoot" null null)))

(fn `UserConstructionScript`
  (bind _monsterclassarray (`self.MonsterClassArray`))
  (`KismetArrayLibrary.Array_Add` _monsterclassarray "/Script/SuperSoldier.SS_Scorobey")
  (`KismetArrayLibrary.Array_Add` _monsterclassarray "/Script/SuperSoldier.SS_Creepster")
  (`KismetArrayLibrary.Array_Add` _monsterclassarray "/Script/SuperSoldier.SS_LandBug")
  (`KismetArrayLibrary.Array_Add` _monsterclassarray "/Script/SuperSoldier.SS_Kraken"))