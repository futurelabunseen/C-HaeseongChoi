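; BP_PrecisionStrike is a rocket projectile that flies at a given location and deals area damage on impact.
; Strike aims it at the target and enables Tick, which sweeps it forward at Speed.
; A blocking hit spawns Niagara explosion and aftermath effects, draws a debug box and damages SSCharacterBase actors overlapping the AttackRange box.
; The rocket then disables collision, hides and destroys itself after a short delay.
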(event `self.ReceiveBeginPlay`)

(event `self.ReceiveTick`
  (params (DeltaSeconds :type "Float (single-precision)"))
  (`self.K2_SetActorLocation` (+ (`self.K2_GetActorLocation`) (* (`self.GetActorForwardVector`) (* DeltaSeconds (`self.Speed`)))) true))

(event `Strike`
  (params (TargetLocation :type "Vector Structure"))
  (`self.K2_SetActorRotation` (`KismetMathLibrary.FindLookAtRotation` (`self.K2_GetActorLocation`) TargetLocation))
  (`self.SetActorTickEnabled` true)
  (`self.SetActorTickEnabled` true))

(event `self.SM_Rocket.OnComponentHit`
  (params (HitComponent :type "PrimitiveComponent Object Reference") (OtherActor :type "Actor Object Reference") (OtherComp :type "PrimitiveComponent Object Reference") (NormalImpulse :type "Vector Structure") (Hit :type "HitResult Structure (by ref)"))
  (bind (_bblockinghit _binitialoverlap _time _distance _location _impactpoint _normal _impactnormal) (`GameplayStatics.BreakHitResult` Hit))
  (bind _attackrange (`self.AttackRange`))
  (if _bblockinghit
    (`self.PlayEffect` _location (`KismetMathLibrary.Conv_VectorToRotator` _impactnormal))
    (`KismetSystemLibrary.DrawDebugBox` (`SceneComponent.K2_GetComponentLocation` _attackrange) (`BoxComponent.BoxExtent` _attackrange) (struct :`R` 1.0 :`A` 1.0) (`SceneComponent.K2_GetComponentRotation` _attackrange) 1.0)
    (for _array_element (`PrimitiveComponent.GetOverlappingActors` (`self.AttackRange`) "/Script/SuperSoldier.SSCharacterBase")
      (`GameplayStatics.ApplyDamage` _array_element 30.0 null self))
    (`PrimitiveComponent.SetCollisionEnabled` (`self.SM_Rocket`) "NoCollision")
    (`self.SetActorHiddenInGame` true)
    (`KismetSystemLibrary.Delay` 1.0))
  (`self.K2_DestroyActor`))

(event `PlayEffect`
  (params (Location :type "Vector Structure") (Rotation :type "Rotator Structure"))
  (`NiagaraFunctionLibrary.SpawnSystemAtLocation` "/Game/RocketAttackFX/FX/Vehicle/NS_RocketVehicle_Explosion.NS_RocketVehicle_Explosion" Location Rotation (10.0 4.0 4.0))
  (`NiagaraFunctionLibrary.SpawnSystemAtLocation` "/Game/RocketAttackFX/FX/Vehicle/NS_RocketVehicle_Aftermath.NS_RocketVehicle_Aftermath" Location Rotation (10.0 4.0 4.0)))

(fn `UserConstructionScript`)