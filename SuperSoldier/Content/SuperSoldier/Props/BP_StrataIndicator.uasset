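; BP_StrataIndicator is a throwable physics prop, apparently an indicator marker that lands where it first hits.
; BeginPlay disables Root collision on the authority and enables it on remotes.
; Throw turns on physics and collision, launches Root along the given direction at a fixed speed, and prints velocity for debugging.
; On component hit, only the authority stops physics and disables collision, freezing the prop in place.
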(event `self.ReceiveBeginPlay`
  (bind _root (`self.Root`))
  (`/Engine/EditorBlueprintResources/ActorMacros.Switch Has Authority`
    (:`Authority`
      (`PrimitiveComponent.SetCollisionEnabled` _root "NoCollision"))
    (:`Remote`
      (`PrimitiveComponent.SetCollisionEnabled` _root "QueryAndPhysics"))))

(event `self.ReceiveTick`
  (params (DeltaSeconds :type "Float (single-precision)")))

(event `Throw`
  (params (Dir :type "Vector Structure"))
  (bind _root (`self.Root`))
  (`PrimitiveComponent.SetSimulatePhysics` _root true)
  (`PrimitiveComponent.SetCollisionEnabled` _root "QueryAndPhysics")
  (`PrimitiveComponent.SetPhysicsLinearVelocity` _root (* Dir 2000.0) false "None")
  (`KismetSystemLibrary.PrintString` (`KismetStringLibrary.Conv_VectorToString` (`self.GetVelocity`))))

(event `self.Root.OnComponentHit`
  (params (HitComponent :type "PrimitiveComponent Object Reference") (OtherActor :type "Actor Object Reference") (OtherComp :type "PrimitiveComponent Object Reference") (NormalImpulse :type "Vector Structure") (Hit :type "HitResult Structure (by ref)"))
  (bind _root (`self.Root`))
  (`/Engine/EditorBlueprintResources/ActorMacros.Switch Has Authority`
    (:`Authority`
      (`PrimitiveComponent.SetSimulatePhysics` _root false)
      (`PrimitiveComponent.SetCollisionEnabled` _root "NoCollision"))))

(fn `UserConstructionScript`)